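; BP_Enemy3 is an enemy Blueprint with a floating health bar that tracks its health and faces the player's camera.
; Each Tick it casts the Healthbar widget component's widget to WBP_EnemyHealth and sets the progress bar to Health divided by MaxHealth.
; It then rotates the component with FindLookAtRotation toward the player camera manager's location, billboarding it in world space.
; The graphs shown contain no damage, movement or AI logic.
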(event `self.ReceiveTick`
  (params (DeltaSeconds :type "Float (single-precision)"))
  (bind _healthbar (`self.Healthbar`))
  (bind _aswbp_enemy_health (cast `/Game/UI/Enemy/WBP_EnemyHealth` (`WidgetComponent.GetWidget` (`self.Healthbar`))))
  (`ProgressBar.SetPercent` (`/Game/UI/Enemy/WBP_EnemyHealth.EnemyHealthBar` _aswbp_enemy_health) (/ (`self.Health`) (`self.MaxHealth`)))
  (`SceneComponent.K2_SetWorldRotation` _healthbar (`KismetMathLibrary.FindLookAtRotation` (`SceneComponent.K2_GetComponentLocation` _healthbar) (`SceneComponent.K2_GetComponentLocation` (`PlayerCameraManager.TransformComponent` (`GameplayStatics.GetPlayerCameraManager` 0)))) false false))

(fn `UserConstructionScript`)