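; Health pickup actor that adds half of the player's max health to their current health when touched.
; An overlap on its Sphere by a Player-tagged actor heals player character 0, with no clamp to max in this graph.
; It activates the Impact effect, sets HasOverlapped to prevent repeat healing, then destroys itself after a short delay.
; Any further overlap during that delay destroys it immediately.
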(event `self.Sphere.OnComponentBeginOverlap`
  (params (OverlappedComponent :type "PrimitiveComponent Object Reference") (OtherActor :type "Actor Object Reference") (OtherComp :type "PrimitiveComponent Object Reference") (OtherBodyIndex :type Integer) (bFromSweep :type Boolean) (SweepResult :type "HitResult Structure (by ref)"))
  ;[1 1 1] Health Power up Code
  (if (not (`self.bHasOverlapped`))
    (if (`self.ActorHasTag` OtherActor "Player")
      (bind _asgame_in_amonth_character (cast `GameInAMonthCharacter` (`GameplayStatics.GetPlayerCharacter` 0)))
      (set `GameInAMonthCharacter.CurrentHealth` (+ (* (`GameInAMonthCharacter.MaxHealth` _asgame_in_amonth_character) 0.5) (`GameInAMonthCharacter.CurrentHealth` _asgame_in_amonth_character)) _asgame_in_amonth_character)
      (`ActorComponent.Activate` (`self.Impact`) true)
      (set `self.bHasOverlapped` true)
      (`KismetSystemLibrary.Delay` 0.2)
      (`self.K2_DestroyActor`))
    (else
      (`self.K2_DestroyActor`))))

(fn `UserConstructionScript`)