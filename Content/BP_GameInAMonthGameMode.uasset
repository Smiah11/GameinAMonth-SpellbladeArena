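; Game mode Blueprint that handles the end-of-game screen for win and lose events.
; OnGameWin and OnGameLose each create a widget for the first player, add it to the viewport, focus it in Game and UI input mode, and show the mouse cursor.
; Both events create the same WBP_WinScreen class, so a loss displays the win screen widget with no outcome passed to it.
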(event `self.OnGameWin`
  (bind _returnvalue (`GameplayStatics.GetPlayerController` 0))
  ;[1 1 1] Game Win
  (bind _returnvalue_2 (`|CreateWidget` "/Game/UI/GameMode/WBP_WinScreen.WBP_WinScreen_C" _returnvalue))
  (`UserWidget.AddToViewport` _returnvalue_2 0)
  (`WidgetBlueprintLibrary.SetInputMode_GameAndUIEx` _returnvalue _returnvalue_2)
  (set `PlayerController.bShowMouseCursor` true _returnvalue))

(event `self.OnGameLose`
  (bind _returnvalue (`GameplayStatics.GetPlayerController` 0))
  (bind _returnvalue_2 (`|CreateWidget` "/Game/UI/GameMode/WBP_WinScreen.WBP_WinScreen_C" _returnvalue))
  (`UserWidget.AddToViewport` _returnvalue_2 0)
  (`WidgetBlueprintLibrary.SetInputMode_GameAndUIEx` _returnvalue _returnvalue_2)
  (set `PlayerController.bShowMouseCursor` true _returnvalue))

(fn `UserConstructionScript`)